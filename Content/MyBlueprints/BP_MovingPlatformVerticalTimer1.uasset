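; Vertical moving platform, named as a timed variant, that moves its Door component when its Trigger component registers a hit.
; The hit plays a timeline that lerps Door's relative location between StartPos and EndPos.
; On finish, the Up flag decides the next step: if set, it is cleared; otherwise a long fixed delay runs, then Up is set and the timeline reverses from its end.
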(event `self.Trigger.OnComponentHit`
  (params (HitComponent :type "PrimitiveComponent Object Reference") (OtherActor :type "Actor Object Reference") (OtherComp :type "PrimitiveComponent Object Reference") (NormalImpulse :type "Vector Structure") (Hit :type "HitResult Structure (by ref)"))
  (bind (_direction _newtrack_0) (`Timeline|Timeline_0` :!label _label)
    (:`Update`
      (`SceneComponent.K2_SetRelativeLocationAndRotation` :`self` (`self.Door`) :`NewLocation` (`KismetMathLibrary.VLerp` (`self.StartPos`) (`self.EndPos`) _newtrack_0)))
    (:`Finished`
      (if (`self.bUp`)
        (set `self.bUp` false)
        (else
          (`KismetSystemLibrary.Delay` 500.0)
          (set `self.bUp` true)
          (goto _label :!via `ReverseFromEnd`))))))

(fn `UserConstructionScript`)