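; BP_TriggerPhysics is an actor with a small box mesh that starts simulating physics when a first-person projectile hits it.
; The Hit event casts the other actor to FirstPersonProjectile and enables physics on SmallBox only on success.
; The construction script gives the box a dynamic material instance from BaseMaterial.
; Logic to randomize that material's DiffuseColor exists but is disconnected, so it never runs.
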(event `self.ReceiveHit`
  (params (MyComp :type "PrimitiveComponent Object Reference") (Other :type "Actor Object Reference") (OtherComp :type "PrimitiveComponent Object Reference") (bSelfMoved :type Boolean) (HitLocation :type "Vector Structure") (HitNormal :type "Vector Structure") (NormalImpulse :type "Vector Structure") (Hit :type "HitResult Structure (by ref)"))
  ;[1 1 1] Physics on the static mesh
  (cast `/Game/FirstPersonBP/Blueprints/FirstPersonProjectile` Other)
  (`PrimitiveComponent.SetSimulatePhysics` (`self.SmallBox`) true))

(fn `UserConstructionScript`
  ;[1 1 1] Chreating the material that the that static mesh have
  (bind _returnvalue (`PrimitiveComponent.CreateDynamicMaterialInstance` (`self.SmallBox`) 0 "/Game/FirstPerson/Meshes/BaseMaterial.BaseMaterial" "None"))
  (set `self.Dynamic Material` _returnvalue))