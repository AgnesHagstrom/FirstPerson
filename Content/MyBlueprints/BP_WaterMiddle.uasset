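; BP_WaterMiddle is a water gate actor that raises or lowers water when its trigger box is hit.
; A boolean picks play or reverse for the gate timeline, whose every update also drives the water timeline the same way.
; The gate lerps from its current location toward the water's BeginPlay location, while the water lerps between two stored positions.
; Each timeline flips the boolean on finishing.
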(event `self.ReceiveBeginPlay`
  (set `self.EndPosGate` (`SceneComponent.RelativeLocation` (`self.Wather`))))

(event `self.TriggerBox.OnComponentHit`
  (params (HitComponent :type "PrimitiveComponent Object Reference") (OtherActor :type "Actor Object Reference") (OtherComp :type "PrimitiveComponent Object Reference") (NormalImpulse :type "Vector Structure") (Hit :type "HitResult Structure (by ref)"))
  (if (`self.bIfWatherISUp`)
    (bind (_direction _watherrising) (`Timeline|Timeline_0` :!via `Reverse` :!label _label)
      (:`Update`
        (`SceneComponent.K2_SetRelativeLocation` (`self.WaterGate`) (`KismetMathLibrary.VLerp` (`SceneComponent.RelativeLocation` (`self.WaterGate`)) (`self.EndPosGate`) _watherrising) false false)
        (if (`self.bIfWatherISUp`)
          (bind (_direction_2 _watherrising_2) (`Timeline|Timeline_1` :!via `Reverse` :!label _label_2)
            (:`Update`
              (`SceneComponent.K2_SetRelativeLocation` (`self.Wather`) (`KismetMathLibrary.VLerp` (`self.StartPosWater`) (`self.EndPosWater`) _watherrising_2) false false))
            (:`Finished`
              (if (`self.bIfWatherISUp`)
                (set `self.bIfWatherISUp` false)
                (else
                  (set `self.bIfWatherISUp` true)))))
          (else
            (goto _label_2))))
      (:`Finished`
        (if (`self.bIfWatherISUp`)
          (set `self.bIfWatherISUp` false)
          (else
            (set `self.bIfWatherISUp` true)))))
    (else
      (goto _label))))

(fn `UserConstructionScript`)