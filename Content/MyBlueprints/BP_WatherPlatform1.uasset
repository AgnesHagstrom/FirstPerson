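; BP_WatherPlatform1 is a platform actor that moves a gate and a water component when its trigger box is hit.
; Any hit plays Timeline_1, which lerps the gate toward EndPosWall.
; Each gate update also calls Play on Timeline_0, which lerps the water toward EndPosWather.
; Both lerps start from the current relative location rather than a cached start, so motion compounds each update.
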(event `self.TriggerBox.OnComponentHit`
  (params (HitComponent :type "PrimitiveComponent Object Reference") (OtherActor :type "Actor Object Reference") (OtherComp :type "PrimitiveComponent Object Reference") (NormalImpulse :type "Vector Structure") (Hit :type "HitResult Structure (by ref)"))
  (bind (_direction _watherrising) (`Timeline|Timeline_1`)
    (:`Update`
      (`SceneComponent.K2_SetRelativeLocationAndRotation` :`self` (`self.Gate`) :`NewLocation` (`KismetMathLibrary.VLerp` (`SceneComponent.RelativeLocation` (`self.Gate`)) (`self.EndPosWall`) _watherrising))
      (bind (_direction_2 _watherrising_2) (`Timeline|Timeline_0`)
        (:`Update`
          (`SceneComponent.K2_SetRelativeLocationAndRotation` :`self` (`self.Wather`) :`NewLocation` (`KismetMathLibrary.VLerp` (`SceneComponent.RelativeLocation` (`self.Wather`)) (`self.EndPosWather`) _watherrising_2)))))))

(fn `UserConstructionScript`)