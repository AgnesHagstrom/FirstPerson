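; BP_Water02 is a Blueprint that moves two gates and a water mesh in sequence when its Trigger component is hit.
; Timelines for the bottom gate, middle gate and water are chained, each starting the next from its Update output through a Delay.
; Each update lerps the mesh from its current relative location toward an end position, so the start point shifts as it moves.
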(event `self.Trigger.OnComponentHit`
  (params (HitComponent :type "PrimitiveComponent Object Reference") (OtherActor :type "Actor Object Reference") (OtherComp :type "PrimitiveComponent Object Reference") (NormalImpulse :type "Vector Structure") (Hit :type "HitResult Structure (by ref)"))
  (bind (_direction _newtrack_0) (`Timeline|GateBottom`)
    (:`Update`
      (`SceneComponent.K2_SetRelativeLocationAndRotation` :`self` (`self.SM_GateBottom`) :`NewLocation` (`KismetMathLibrary.VLerp` (`SceneComponent.RelativeLocation` (`self.SM_GateBottom`)) (`self.EndPosBottom`) _newtrack_0))
      (`KismetSystemLibrary.Delay` 1.0)
      (bind (_direction_2 _newtrack_0_2) (`Timeline|GateMiddle`)
        (:`Update`
          (`SceneComponent.K2_SetRelativeLocationAndRotation` :`self` (`self.SM_GateMiddle`) :`NewLocation` (`KismetMathLibrary.VLerp` (`SceneComponent.RelativeLocation` (`self.SM_GateMiddle`)) (`self.EndPosMiddle`) _newtrack_0_2))
          (`KismetSystemLibrary.Delay` 2.0)
          (bind (_direction_3 _newtrack_0_3) (`Timeline|Water`)
            (:`Update`
              (`SceneComponent.K2_SetRelativeLocationAndRotation` :`self` (`self.SM_WaterMesh`) :`NewLocation` (`KismetMathLibrary.VLerp` (`SceneComponent.RelativeLocation` (`self.SM_WaterMesh`)) (`self.EndPosWater`) _newtrack_0_3)))))))))

(fn `UserConstructionScript`)