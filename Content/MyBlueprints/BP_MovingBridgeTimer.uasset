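; BP_MovingBridgeTimer is a bridge actor that swings open or closed when hit, then returns on a timer.
; The Hit event plays the MovingPlatform timeline, which lerps the static mesh's relative rotation through 90 degrees.
; When the timeline finishes, a fixed delay precedes reversing it, with the IsRotated flag stopping the cycle once the return completes.
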(event `self.ReceiveHit`
  (params (MyComp :type "PrimitiveComponent Object Reference") (Other :type "Actor Object Reference") (OtherComp :type "PrimitiveComponent Object Reference") (bSelfMoved :type Boolean) (HitLocation :type "Vector Structure") (HitNormal :type "Vector Structure") (NormalImpulse :type "Vector Structure") (Hit :type "HitResult Structure (by ref)"))
  (`self.EnableInput` null)
  (bind (_direction _newtrack_0) (`Timeline|MovingPlatform` :!label _label)
    (:`Update`
      (`SceneComponent.K2_SetRelativeRotation` (`self.StaticMesh`) (`KismetMathLibrary.RLerp` (struct) (struct :`Yaw` 90.0) _newtrack_0) false false))
    (:`Finished`
      (if (`self.bIsRotated`)
        (set `self.bIsRotated` false)
        (else
          (`KismetSystemLibrary.Delay` 5.0)
          (set `self.bIsRotated` true)
          (goto _label :!via `Reverse`))))))

(fn `UserConstructionScript`)